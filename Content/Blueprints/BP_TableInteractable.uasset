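; BP_TableInteractable is a table interactable with a progress bar and a task bubble, both shown through widget components.
; On BeginPlay it registers itself as the progress bar widget's Interactable and hides both widgets, stopping early if the BP_ProgressBar cast fails.
; Show and hide events toggle each widget's visibility, and ShowProgressBar also calls the parent implementation after revealing the bar.
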(event EventBeginPlay
  ;[1 1 1] Hide Progress Bar When Game Starts
  (bind _asbp_progress_bar (Utilities|Casting|CastToBP_ProgressBar (UserInterface|GetUserWidgetObject (Variables|Default|GetProgressBar))))
  (Variables|/Game/Widgets/BP_ProgressBar.BP_ProgressBar_C|SetInteractable _asbp_progress_bar self)
  (Widget|SetVisibility (UserInterface|GetUserWidgetObject (Variables|Default|GetProgressBar)) "Hidden")
  ;[1 1 1] Hide Task Bubble When Game Starts
  (Widget|SetVisibility (UserInterface|GetUserWidgetObject (Variables|Default|GetTaskBubble)) "Hidden"))

(event EventShowTaskBubble
  ;[1 1 1] Show Task Bubble
  (Widget|SetVisibility (UserInterface|GetUserWidgetObject (Variables|Default|GetTaskBubble)) "Visible"))

(event EventHideTaskBubble
  ;[1 1 1] Hide Task Bubble
  (Widget|SetVisibility (UserInterface|GetUserWidgetObject (Variables|Default|GetTaskBubble)) "Hidden"))

(event EventShowProgressBar
  ;[1 1 1] Show Progress Bar
  (Widget|SetVisibility (UserInterface|GetUserWidgetObject (Variables|Default|GetProgressBar)) "Visible")
  (|CallParentFunction))

(event EventHideProgressBar
  ;[1 1 1] Hide Progress Bar
  (Widget|SetVisibility (UserInterface|GetUserWidgetObject (Variables|Default|GetProgressBar)) "Hidden"))

(fn ConstructionScript)