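; Task controller that periodically hands out random tasks to the BP_TableInteractable actors in the level.
; BeginPlay gathers the tables and starts a looping timer that picks one at random, activates its task and shows its bubble.
; Assignment is gated by task count and the table's repeat limits, recursively re-rolling when the pick is already active.
; Debug prints trace selections, and PrintArrayLength also sets the table count used by that gate.
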(event Custom|AssignNewRandomTask
  (bind (_selectedarrayelement _indexofselectedarrayelement) (CallFunction|GetRandomArrayElement (Variables|Default|GetInteractablesArrayQueue)))
  (Variables|Default|SetSelectedInteractable _selectedarrayelement)
  (bind _returnvalue (CallFunction|CanAssignNewTask))
  (if _returnvalue
    (if (Variables|/Script/MyProject2.Interactable|GetisTaskActive (Variables|Default|GetSelectedInteractable))
      (CallFunction|PrintObjectNameandIndexRed (Variables|Default|GetSelectedInteractable) _indexofselectedarrayelement)
      (CallFunction|AssignNewRandomTask)
      (else
        (CallFunction|PrintObjectNameandIndex (Variables|Default|GetSelectedInteractable) _indexofselectedarrayelement)
        (Variables|/Script/MyProject2.Interactable|SetisTaskActive (Variables|Default|GetSelectedInteractable) true)
        (Class|Interactable|ShowTaskBubble (Variables|Default|GetSelectedInteractable))
        (Variables|Default|SetTaskCounter (+ (Variables|Default|GetTaskCounter) 1))))
    (else
      (Development|PrintString "Maximum Number Of Tasks Reached" true true "(R=1.000000,G=1.000000,B=0.000000,A=1.000000)" 5.0))))

(event EventBeginPlay
  (bind _outactors (Actor|GetAllActorsOfClass "/Game/Blueprints/BP_TableInteractable.BP_TableInteractable_C"))
  (Variables|Default|SetInteractablesArray _outactors)
  (bind _output_get (Variables|Default|SetInteractablesArrayQueue _outactors))
  (CallFunction|PrintAllArrayElements _output_get)
  (CallFunction|PrintArrayLength _output_get)
  (Utilities|Time|SetTimerbyEvent (delegate Custom|AssignNewRandomTask) 3.0 true))

(event Collision|EventActorBeginOverlap
  (params (OtherActor :type Actor%20Object%20Reference)))

(event EventTick
  (params (DeltaSeconds :type Float%20%28single-precision%29)))

(fn ConstructionScript)

(fn PrintAllArrayElements
  (params (Array :type Array%20of%20BP%20Table%20Interactable%20Object%20References))
  (for (_array_element _array_index) Array
    (Development|PrintString (Utilities|String|Append (Utilities|GetDisplayName _array_element) " --- Index is " (Utilities|String|ToString(Integer) _array_index)) true true "(R=0.000000,G=0.660000,B=1.000000,A=1.000000)" 5e+01)))

(fn PrintArrayLength
  (params (Array :type Array%20of%20BP%20Table%20Interactable%20Object%20References))
  (bind _returnvalue (Utilities|Array|Length Array))
  (Variables|Default|SetNumberOfInteractables _returnvalue)
  (Development|PrintString (Utilities|String|Append "Array Length is: " (Utilities|String|ToString(Integer) _returnvalue)) true true "(R=0.000000,G=0.660000,B=1.000000,A=1.000000)" 5e+01))

(fn GetRandomArrayElement
  (params (Array :type Array%20of%20BP%20Table%20Interactable%20Object%20References))
  (bind _output_get (Variables|Default|SetRandom%20Number (Math|Random|RandomInteger (Utilities|Array|Length Array))))
  (bind _asbp_table_interactable (Utilities|Casting|CastToBP_TableInteractable (Utilities|Array|Get(acopy) Array _output_get))
    (:then
      (return _asbp_table_interactable _output_get))
    (:CastFailed
      (Development|PrintString "Failed to get a refference" true true "(R=1.000000,G=0.000000,B=0.000000,A=1.000000)" 2e+01))))

(fn PrintObjectNameandIndex
  (params (ObjectRefference :type BP%20Table%20Interactable%20Object%20Reference) (Index :type Integer))
  (Development|PrintString (Utilities|String|Append "Selected Index Is:" (Utilities|String|ToString(Integer) Index)) true true "(R=0.000000,G=1.000000,B=0.000000,A=1.000000)" 6e+01)
  (Development|PrintString (Utilities|GetDisplayName ObjectRefference) true true "(R=0.000000,G=1.000000,B=0.000000,A=1.000000)" 6e+01))

(fn GetRandomArrayElementandShowTask
  (params (Array :type Array%20of%20BP%20Table%20Interactable%20Object%20References))
  (bind (_selectedarrayelement _indexofselectedarrayelement) (CallFunction|GetRandomArrayElement Array))
  (CallFunction|PrintObjectNameandIndex _selectedarrayelement _indexofselectedarrayelement)
  (Class|Interactable|ShowTaskBubble _selectedarrayelement))

(fn PrintObjectNameandIndexRed
  (params (ObjectRefference :type BP%20Table%20Interactable%20Object%20Reference) (Index :type Integer))
  (Development|PrintString (Utilities|String|Append "Selected Index Is:" (Utilities|String|ToString(Integer) Index)) true true "(R=1.000000,G=0.000000,B=0.000000,A=1.000000)" 6e+01)
  (Development|PrintString (Utilities|GetDisplayName ObjectRefference) true true "(R=1.000000,G=0.000000,B=0.000000,A=1.000000)" 6e+01))

(fn CanAssignNewTask
  (bind _selectedinteractable (Variables|Default|GetSelectedInteractable))
  (bind _taskcounter (Variables|Default|GetTaskCounter))
  (bind _taskcompletedcount (Variables|/Script/MyProject2.Interactable|GetTaskCompletedCount _selectedinteractable))
  (bind _istaskrepeatable (Variables|/Script/MyProject2.Interactable|GetIsTaskRepeatable _selectedinteractable))
  (Development|PrintString (Utilities|String|Append "TaskCount is " (Utilities|String|ToString(Integer) _taskcounter)) true true "(R=1.000000,G=1.000000,B=0.000000,A=1.000000)")
  (return (and (and (< _taskcounter (Variables|Default|GetMaxTaskNumber)) (< _taskcounter (Variables|Default|GetNumberOfInteractables))) (or (and (not _istaskrepeatable) (== _taskcompletedcount 0)) (and _istaskrepeatable (< _taskcompletedcount (Variables|/Script/MyProject2.Interactable|GetMaxRepeatableTask _selectedinteractable)))))))